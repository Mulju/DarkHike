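; Controller for a lamb that switches it between waiting, grazing and following, and enables player input only for the "Quest Lamb".
; On Interact, the lamb waits, then follows and destroys the tagged LambCage if the player is nearby with a dandelion in inventory; otherwise it returns to grazing.
; Once ClearReached is set, Tick sends it to the sacrifice zone if it is alive and marked ToSacrifice, or to the wait zone if unmarked.
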(event EventTick
  (params (DeltaSeconds :type Float%20%28single-precision%29))
  (Utilities|FlowControl|Sequence
    (:then_0
      (bind _ctrldlamb (Variables|Default|GetCtrldLamb)
        (:then
          (if true
            (if (Variables|/Script/DarkHike.Lamb|GetbClearReached _ctrldlamb)
              (if (Variables|/Script/DarkHike.Lamb|GetbToSacrifice _ctrldlamb)
                (if (Variables|Default|GetbAlive)
                  (Class|LambController|MovetoSacrificeZone))
                (else
                  (Class|LambController|MovetoWaitZone))))))
        (:else)))))

(event EventBeginPlay
  (Utilities|FlowControl|Sequence
    (:then_0
      (bind _ctrldlamb (Variables|Default|GetCtrldLamb)
        (:then
          (if (Utilities|Enum|Equal(Enum) (Variables|/Script/DarkHike.Lamb|GetLambName _ctrldlamb) "Quest Lamb")
            (Input|EnableInput (Game|GetPlayerController 0))
            (Development|PrintString "Lamb Input Enabled")))
        (:else
          (Development|PrintString "Lamb reference not valid" false))))
    (:then_1
      (bind _outactors (Actor|GetAllActorswithTag "LambCage"))
      (bind _asbp_lamb_cage (Utilities|Casting|CastToBP_LambCage (Utilities|Array|Get(acopy) _outactors)))
      (Variables|Default|SetLambCage _asbp_lamb_cage))))

(event Input|ActionEvents|InputActionInteract
  (params (Key :type Key%20Structure :default "None"))
  (:Pressed
    (bind _ctrldlamb (Variables|Default|GetCtrldLamb)
      (:then
        (if (not (Variables|/Script/DarkHike.Lamb|GetbClearReached _ctrldlamb))
          (Class|LambController|StateWait)
          (bind _ctrldlamb_2 (Variables|Default|GetCtrldLamb)
            (:then
              (if (<= (Transformation|GetDistanceTo (Game|GetPlayerCharacter 0) _ctrldlamb_2) 375.0)
                (bind _asbp_player (Utilities|Casting|CastToBP_Player (Game|GetPlayerCharacter 0)))
                (if (.bSuccess (Default|QueryInventory (Variables|/Game/Code/Character/BP_Player.BP_Player_C|GetKeyItemInventory _asbp_player) "dandelion" 1))
                  (Class|LambController|StateFollow)
                  (bind _lambcage (Variables|Default|GetLambCage)
                    (:then
                      (Actor|DestroyActor _lambcage))
                    (:else))
                  (else
                    (Utilities|FlowControl|Delay 6.0)
                    (Class|LambController|StateGraze)))
                (else
                  (Class|LambController|StateGraze))))
            (:else))))
      (:else))))

(fn ConstructionScript)