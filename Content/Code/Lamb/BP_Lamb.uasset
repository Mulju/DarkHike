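; BP_Lamb is a lamb actor that activates the level's altar when it reaches its goal zone.
; On overlap with the actor referenced by ClearZone, it sets ClearReached and looks up all BP_altar actors.
; It sets IsLambActivated on the altar only when exactly one exists, and prints debug messages for goal and non-goal overlaps.
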(event EventBeginPlay)

(event Collision|EventActorBeginOverlap
  (params (OtherActor :type Actor%20Object%20Reference))
  (if (== (Variables|Default|GetClearZone) OtherActor)
    (Development|PrintString "Collided with goal")
    (Variables|Default|SetbClearReached true)
    (bind _outactors (Actor|GetAllActorsOfClass "/Game/Blueprints/3D-models/Props/Medium/altar/BP_altar.BP_altar_C"))
    (if (== (Utilities|Array|Length _outactors) 1)
      (Variables|/Script/DarkHike.Altar|SetbIsLambActivated (Utilities|Array|Get(acopy) _outactors) true))
    (else
      (Development|PrintString "Collided with something else" false))))

(event EventTick
  (params (DeltaSeconds :type Float%20%28single-precision%29)))

(fn ConstructionScript)