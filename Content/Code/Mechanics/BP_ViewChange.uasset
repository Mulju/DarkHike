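; BP_ViewChange is a trigger volume that temporarily moves the player's camera view to this actor.
; When active, a BP_Player overlap eases the view here, holds for a set duration, then blends back to the controlled pawn.
; During the shot it either slows walk speed or disables input, applied before the player class check, then restores it.
; A gate closes after the sequence when the trigger is one-time.
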(event OnComponentBeginOverlap(Box)
  (params (OverlappedComponent :type Primitive%20Component%20Object%20Reference) (OtherActor :type Actor%20Object%20Reference) (OtherComp :type Primitive%20Component%20Object%20Reference) (OtherBodyIndex :type Integer) (bFromSweep :type Boolean) (SweepResult :type Hit%20Result%20Structure%20%28by%20ref%29))
  (bind _returnvalue (Game|GetPlayerController 0))
  (bind _blendtimefromplayer (Variables|Default|GetBlendTimeFromPlayer))
  (bind _blendtimetoplayer (Variables|Default|GetBlendTimeToPlayer))
  (Utilities|FlowControl|Gate false :!label _label
    (:Exit
      (if (Variables|Default|GetbIsWalking)
        (Variables|/Script/Engine.CharacterMovementComponent|SetMaxWalkSpeed (Variables|/Script/Engine.Character|GetCharacterMovement (Game|GetPlayerCharacter 0)) 5e+01)
        (else
          (Input|DisableInput OtherActor (Game|GetPlayerController 0))))
      (if (Utilities|ClassIsChildOf (Utilities|GetClass OtherActor) "/Game/Code/Character/BP_Player.BP_Player_C")
        (Game|Player|SetViewTargetwithBlend (Game|GetPlayerController 0) self _blendtimefromplayer "VTBlend_EaseInOut" (Variables|Default|GetBlendVariable) false)
        (Utilities|FlowControl|Delay (/ _blendtimefromplayer 2.0))
        (Utilities|FlowControl|Delay (Variables|Default|GetBlendTimeFromPlayer))
        (Utilities|FlowControl|Delay (Variables|Default|GetStayDuration))
        (Game|Player|SetViewTargetwithBlend _returnvalue (Pawn|GetControlledPawn _returnvalue) _blendtimetoplayer "VTBlend_EaseInOut" (Variables|Default|GetBlendVariable) false)
        (Utilities|FlowControl|Delay (/ _blendtimetoplayer 2.0))
        (Utilities|FlowControl|Delay (/ (Variables|Default|GetBlendTimeToPlayer) 2.0))
        (if (Variables|Default|GetbIsWalking)
          (Variables|/Script/Engine.CharacterMovementComponent|SetMaxWalkSpeed (Variables|/Script/Engine.Character|GetCharacterMovement (Game|GetPlayerCharacter 0)) 6e+02)
          (else
            (Input|EnableInput OtherActor (Game|GetPlayerController 0))))
        (if (Variables|Default|GetbIsOneTime)
          (goto _label Close))))))

(event EventBeginPlay
  (if (Variables|Default|GetbIsActive)
    (Collision|SetCollisionProfileName (Variables|Default|GetBox) "OverlapAllDynamic" true :!class /Script/Engine.PrimitiveComponent)
    (else
      (Collision|SetCollisionProfileName (Variables|Default|GetBox) "NoCollision" true :!class /Script/Engine.PrimitiveComponent))))

(event Collision|EventActorBeginOverlap
  (params (OtherActor :type Actor%20Object%20Reference)))

(event EventTick
  (params (DeltaSeconds :type Float%20%28single-precision%29)))

(fn ConstructionScript)