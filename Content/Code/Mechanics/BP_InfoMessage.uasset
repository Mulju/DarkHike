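; BP_InfoMessage is a trigger volume that displays its Message text through the W_InfoMessage widget.
; Shortly after BeginPlay it caches the first top-level instance of that widget, rather than creating one.
; Any overlap with its Box calls ShowMessage, with no check on the overlapping actor.
; When IsMazeInfo is set, HasBeenShown limits the message to one showing; otherwise it repeats on every overlap.
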(event OnComponentBeginOverlap(Box)
  (params (OverlappedComponent :type Primitive%20Component%20Object%20Reference) (OtherActor :type Actor%20Object%20Reference) (OtherComp :type Primitive%20Component%20Object%20Reference) (OtherBodyIndex :type Integer) (bFromSweep :type Boolean) (SweepResult :type Hit%20Result%20Structure%20%28by%20ref%29))
  (if (Variables|Default|GetbIsMazeInfo)
    (if (not (Variables|Default|GetbHasBeenShown))
      (Default|ShowMessage (Variables|Default|GetInfoMessage) (Variables|Default|GetMessage))
      (Variables|Default|SetbHasBeenShown true))
    (else
      (Default|ShowMessage (Variables|Default|GetInfoMessage) (Variables|Default|GetMessage)))))

(event EventBeginPlay
  (Utilities|FlowControl|Delay 0.2)
  (bind _foundwidgets (Widget|GetAllWidgetsOfClass "/Game/Blueprints/UI-Widgets/W_InfoMessage.W_InfoMessage_C" true))
  (Variables|Default|SetInfoMessage (Utilities|Array|Get(acopy) _foundwidgets)))

(fn ConstructionScript)