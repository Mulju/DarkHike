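; BP_EndSequence is a sphere trigger that runs the game's ending when the player overlaps it.
; It flags BP_Player as at the end, disables input and rotates the player's mesh to face the actor's root, noted as the hole.
; After a fixed delay it restores input, switches to UI-only mode with a visible cursor, marks GI_DarkHike as ended and opens the main menu map.
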(event OnComponentBeginOverlap(Sphere)
  (params (OverlappedComponent :type Primitive%20Component%20Object%20Reference) (OtherActor :type Actor%20Object%20Reference) (OtherComp :type Primitive%20Component%20Object%20Reference) (OtherBodyIndex :type Integer) (bFromSweep :type Boolean) (SweepResult :type Hit%20Result%20Structure%20%28by%20ref%29))
  (bind _returnvalue (Game|GetPlayerController 0))
  ;[1 1 1] Turn the player towards the hole
  (bind _asbp_player (Utilities|Casting|CastToBP_Player OtherActor))
  (Variables|/Game/Code/Character/BP_Player.BP_Player_C|SetbIsAtEnd _asbp_player true)
  (Input|DisableInput _asbp_player _returnvalue)
  (Components|MoveComponentTo (Variables|/Script/Engine.Character|GetMesh _asbp_player) "0.000000,0.000000,-34.000000" (Math|Rotator|MakeRotator 0.0 0.0 (- (.yaw (Math|Rotator|FindLookatRotation (Transformation|GetActorLocation OtherActor) (Transformation|GetWorldLocation (Variables|Default|GetDefaultSceneRoot)))) (.yaw (Transformation|GetWorldRotation (Variables|/Script/Engine.Character|GetCapsuleComponent _asbp_player))))) false false 0.2 true)
  (Utilities|FlowControl|Delay 2e+01)
  (Input|EnableInput _asbp_player _returnvalue)
  (Input|SetInputModeUIOnly _returnvalue 0 "DoNotLock" false)
  (Variables|/Script/Engine.PlayerController|SetbShowMouseCursor _returnvalue true)
  (bind _asgi_dark_hike (Utilities|Casting|CastToGI_DarkHike (Game|GetGameInstance)))
  (Variables|/Game/Code/GI_DarkHike.GI_DarkHike_C|SetbGameEnded _asgi_dark_hike true)
  (Game|OpenLevel(byObjectReference) "/Game/Maps/Menus/MainMenuMap.MainMenuMap"))

(fn ConstructionScript)