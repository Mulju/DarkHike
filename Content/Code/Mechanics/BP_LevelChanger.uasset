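; BP_LevelChanger is a level-transition trigger that preserves the player's inventory in the game instance.
; When BP_Player overlaps InteractComp, it copies the collectible and key item inventory contents into GI_DarkHike.
; Disconnected logic would set LevelToLoad to a normal or EVIL C3_prop variant from GoodBadScore when IsL2 is set.
; The graph itself contains no level-loading call.
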(event OnComponentBeginOverlap(InteractComp)
  (params (OverlappedComponent :type Primitive%20Component%20Object%20Reference) (OtherActor :type Actor%20Object%20Reference) (OtherComp :type Primitive%20Component%20Object%20Reference) (OtherBodyIndex :type Integer) (bFromSweep :type Boolean) (SweepResult :type Hit%20Result%20Structure%20%28by%20ref%29))
  (bind _asbp_player (Utilities|Casting|CastToBP_Player OtherActor))
  (bind _asgi_dark_hike (Utilities|Casting|CastToGI_DarkHike (Game|GetGameInstance)))
  (Variables|/Game/Code/GI_DarkHike.GI_DarkHike_C|SetCollectibleInventoryContent _asgi_dark_hike (Variables|/Game/Code/Mechanics/Inventory/InventorySystem.InventorySystem_C|GetContent (Variables|/Game/Code/Character/BP_Player.BP_Player_C|GetInventorySystem _asbp_player)))
  (Variables|/Game/Code/GI_DarkHike.GI_DarkHike_C|SetKeyInventoryContent _asgi_dark_hike (Variables|/Game/Code/Mechanics/Inventory/InventorySystem.InventorySystem_C|GetContent (Variables|/Game/Code/Character/BP_Player.BP_Player_C|GetKeyItemInventory _asbp_player))))

(fn ConstructionScript)