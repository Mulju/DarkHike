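; Player character that can walk on the walls of "Labyrinth"-tagged maze geometry when CanWallWalk is set.
; Move inputs run line traces to detect walls and edges, then MoveComponentTo shifts capsule and mesh into Flying movement, and StopOnWall restores Falling.
; Tick aligns the mesh to the surface normal and toggles blood-lake ripples by physical material.
; Also handles pause menu, inventory HUD, level reload and a mesh-following audio listener.
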(event EventBeginPlay
  (bind _playerears (Variables|Default|GetPlayerEars))
  (Utilities|FlowControl|Sequence
    (:then_0
      (Variables|/Game/Code/Mechanics/Inventory/InventorySystem.InventorySystem_C|SetPlayerMesh (Variables|Default|GetInventorySystem) (Variables|Character|GetMesh))
      (bind _returnvalue (UserInterface|CreateWidget "/Game/Blueprints/UI-Widgets/Inventory/W_PlayerHUD.W_PlayerHUD_C"))
      (bind _output_get (Variables|Default|SetHUD _returnvalue))
      (UserInterface|Viewport|AddtoViewport _output_get 0))
    (:then_1
      ;[1 1 1] Ears Rotate with Mesh forward
      (Class|PlayerController|SetAudioListenerOverride (Game|GetPlayerController (Variables|/Script/Engine.Pawn|GetPlayerState (Game|GetPlayerCharacter 0))) _playerears "0, 0, 0" (Transformation|GetWorldRotation _playerears)))))

(event EventTick
  (params (DeltaSeconds :type Float%20%28single-precision%29))
  (bind _returnvalue (Transformation|GetVelocity))
  (bind _mesh (Variables|Character|GetMesh))
  (bind _returnvalue_2 (Transformation|GetWorldTransform _mesh))
  (Utilities|FlowControl|Sequence
    (:then_0
      ;[1 1 1] Set the closes actor value from code to InventorySystem blueprint
      (Variables|/Game/Code/Mechanics/Inventory/InventorySystem.InventorySystem_C|SetCodeClosestActor (Variables|Default|GetInventorySystem) (Variables|Default|GetClosestActor))
      (if (Variables|Default|GetbOnWall)
        (if (not (Variables|Default|GetbInTransition))
          (bind (_returnvalue_3 _outhit) (Utilities|FloorCheck))
          (if _returnvalue_3
            (Transformation|SetWorldLocationAndRotation _mesh (Math|Vector|Lerp(Vector) (.location _returnvalue_2) (.Location (Collision|BreakHitResult _outhit)) 0.1) (Math|Rotator|Lerp(Rotator) (.rotation _returnvalue_2) (Math|Rotator|MakeRotfromZX (.Normal (Collision|BreakHitResult _outhit)) (Math|Vector|Normalize _returnvalue)) (Math|Float|SelectFloat 0.5 0.0 (> (Math|Vector|VectorLength _returnvalue) 0.0)) true) false false)))))
    (:then_1
      (bind _outhit_2 (Collision|LineTraceByChannel (Transformation|GetWorldLocation (Variables|Character|GetMesh self)) "0.000000,0.000000,300.000000" "TraceTypeQuery1" false 0 "None"))
      (Utilities|IsValid (.PhysMat (Collision|BreakHitResult _outhit_2))
        (:Is%20Valid
          (if (== (.PhysMat (Collision|BreakHitResult _outhit_2)) "/Game/Audio/PMAT_AudioSurfaces/PMAT_BloodLake.PMAT_BloodLake")
            (if (not (Components|Activation|IsActive (Variables|Default|GetBloodLakeRiple)))
              (Utilities|FlowControl|Delay 0.18)
              (Components|Activation|Activate (Variables|Default|GetBloodLakeRiple) false))
            (elif (Components|Activation|IsActive (Variables|Default|GetBloodLakeRiple))
              (Components|Activation|Deactivate (Variables|Default|GetBloodLakeRiple)))))))))

(event Input|ActionEvents|InputActionInventory
  (params (Key :type Key%20Structure :default "None"))
  (:Pressed
    (if (not (Variables|Default|GetbIsPaused))
      (Default|DisplayPlayerInventory (Variables|Default|GetHUD)))))

(event Input|AxisEvents|InputAxisMoveForward
  (params (AxisValue :type Float%20%28single-precision%29))
  (if (!= AxisValue 0.0)
    (if (not (Variables|Default|GetbInTransition))
      (if (Variables|Default|GetbCanWallWalk) ; Inside the maze?
        (bind _returnvalue (Utilities|FloorCheck))
        (if _returnvalue
          (|ToFWall AxisValue
            (:Completed
              (if (Variables|Default|GetbOnWall)
                (|WallMoveForward AxisValue)
                (else
                  (if (> (Math|Float|Absolute(Float) AxisValue) (Variables|Default|GetControllerThreshold)) :!label _label
                    (Pawn|Input|AddMovementInput (Math|Vector|GetForwardVector (Math|Rotator|MakeRotator 0.0 0.0 (.Yaw (Math|Rotator|BreakRotator (Pawn|GetControlRotation :!class /Script/Engine.Pawn))))) AxisValue false))))))
          (else
            (Utilities|MovetoWallOuterEdge)))
        (else
          (goto _label))))))

(event Input|AxisEvents|InputAxisMoveRight
  (params (AxisValue :type Float%20%28single-precision%29))
  (if (!= AxisValue 0.0)
    (if (not (Variables|Default|GetbInTransition))
      (if (Variables|Default|GetbCanWallWalk) ; Inside the maze?
        (bind _returnvalue (Utilities|FloorCheck))
        (if _returnvalue
          (|ToRWall
            (:Completed
              (if (Variables|Default|GetbOnWall)
                (|WallMoveRight AxisValue)
                (else
                  (if (> (Math|Float|Absolute(Float) AxisValue) (Variables|Default|GetControllerThreshold)) :!label _label
                    (Pawn|Input|AddMovementInput (Math|Vector|GetRightVector (Math|Rotator|MakeRotator 0.0 0.0 (.Yaw (Math|Rotator|BreakRotator (Pawn|GetControlRotation :!class /Script/Engine.Pawn))))) AxisValue false))))))
          (else
            (Utilities|MovetoWallOuterEdge)))
        (else
          (goto _label))))))

(event Input|KeyboardEvents|Escape
  (params (Key :type Key%20Structure :default "None"))
  (bind _returnvalue (Game|GetPlayerController 0))
  (bind _returnvalue_2 (Game|GetPlayerController 0))
  (:Pressed
    (Development|PrintString (Utilities|String|ToString(Boolean) (Variables|Default|GetbIsPaused)))
    (if (Variables|Default|GetbIsPaused)
      (Utilities|IsValid (Variables|Default|GetPauseMenu)
        (:Is%20Valid
          (bind _aspause_menu (Utilities|Casting|CastToPauseMenu (Variables|Default|GetPauseMenu)))
          (Utilities|IsValid (Variables|/Game/Blueprints/UI-Widgets/Menus/PauseMenu.PauseMenu_C|GetOptionsMenuWidget _aspause_menu)
            (:Is%20Valid
              (Widget|RemovefromParent (Variables|/Game/Blueprints/UI-Widgets/Menus/PauseMenu.PauseMenu_C|GetOptionsMenuWidget _aspause_menu)))
            (:Is%20Not%20Valid
              _))
          (Widget|RemovefromParent (Variables|Default|GetPauseMenu))
          (Variables|Default|SetPauseMenu 0)
          (Variables|Default|SetbIsPaused false)
          (Variables|/Script/Engine.PlayerController|SetbShowMouseCursor _returnvalue false)
          (Input|SetInputModeGameOnly _returnvalue false)
          (Input|SetIgnoreMoveInput _returnvalue false)))
      (else
        (bind _returnvalue_3 (UserInterface|CreateWidget "/Game/Blueprints/UI-Widgets/Menus/PauseMenu.PauseMenu_C" (Game|GetPlayerController 0)))
        (bind _output_get (Variables|Default|SetPauseMenu _returnvalue_3))
        (UserInterface|Viewport|AddtoViewport _output_get 0)
        (Variables|Default|SetbIsPaused true)
        (bind _aspause_menu_2 (Utilities|Casting|CastToPauseMenu (Variables|Default|GetPauseMenu)))
        (Variables|/Game/Blueprints/UI-Widgets/Menus/PauseMenu.PauseMenu_C|SetPlayerReference _aspause_menu_2 self)
        (Variables|/Script/Engine.PlayerController|SetbShowMouseCursor _returnvalue_2 true)
        (Input|SetInputModeGameandUI _returnvalue_2 0 "DoNotLock" true false)
        (Input|SetIgnoreMoveInput _returnvalue_2 true)
        (Settings|GetGameUserSettings)))))

(event Input|KeyboardEvents|P
  (params (Key :type Key%20Structure :default "None"))
  (:Pressed
    (bind _returnvalue (Game|GetCurrentLevelName true))
    (Game|OpenLevel(byName) (Utilities|String|StringToName _returnvalue))))

(event Input|KeyboardEvents|H
  (params (Key :type Key%20Structure :default "None"))
  (bind _returnvalue (Game|GetPlayerController 0))
  (bind _returnvalue_2 (Game|GetPlayerController 0))
  (:Pressed
    (Development|PrintString (Utilities|String|ToString(Boolean) (Variables|Default|GetbIsPaused)))
    (if (Variables|Default|GetbIsPaused)
      (Utilities|IsValid (Variables|Default|GetPauseMenu)
        (:Is%20Valid
          (bind _aspause_menu (Utilities|Casting|CastToPauseMenu (Variables|Default|GetPauseMenu)))
          (Utilities|IsValid (Variables|/Game/Blueprints/UI-Widgets/Menus/PauseMenu.PauseMenu_C|GetOptionsMenuWidget _aspause_menu)
            (:Is%20Valid
              (Widget|RemovefromParent (Variables|/Game/Blueprints/UI-Widgets/Menus/PauseMenu.PauseMenu_C|GetOptionsMenuWidget _aspause_menu)))
            (:Is%20Not%20Valid
              _))
          (Widget|RemovefromParent (Variables|Default|GetPauseMenu))
          (Variables|Default|SetPauseMenu 0)
          (Variables|Default|SetbIsPaused false)
          (Variables|/Script/Engine.PlayerController|SetbShowMouseCursor _returnvalue false)
          (Input|SetInputModeGameOnly _returnvalue false)
          (Input|SetIgnoreMoveInput _returnvalue false)))
      (else
        (bind _returnvalue_3 (UserInterface|CreateWidget "/Game/Blueprints/UI-Widgets/Menus/PauseMenu.PauseMenu_C" (Game|GetPlayerController 0)))
        (bind _output_get (Variables|Default|SetPauseMenu _returnvalue_3))
        (UserInterface|Viewport|AddtoViewport _output_get 0)
        (Variables|Default|SetbIsPaused true)
        (bind _aspause_menu_2 (Utilities|Casting|CastToPauseMenu (Variables|Default|GetPauseMenu)))
        (Variables|/Game/Blueprints/UI-Widgets/Menus/PauseMenu.PauseMenu_C|SetPlayerReference _aspause_menu_2 self)
        (Variables|/Script/Engine.PlayerController|SetbShowMouseCursor _returnvalue_2 true)
        (Input|SetInputModeGameandUI _returnvalue_2 0 "DoNotLock" true false)
        (Input|SetIgnoreMoveInput _returnvalue_2 true)
        (Settings|GetGameUserSettings)))))

(fn ConstructionScript)