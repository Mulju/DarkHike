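; Main menu audio player actor that plays the menu theme track on a loop with soft fades.
; BeginPlay starts the MMThemeTrack audio component with a fade-in.
; Its playback-percent event fades the track out near the end, and its finished event restarts it with another fade-in after a short delay.
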(event OnAudioFinished(MM_ThemeTrack)
  (bind _mm_themetrack (Variables|Default|GetMM_ThemeTrack))
  (Utilities|FlowControl|Delay 6.5)
  (Audio|Components|Audio|Play _mm_themetrack 0.0)
  (Audio|Components|Audio|FadeIn _mm_themetrack 4.0 1.0 0.0 "Linear" :!class /Script/Engine.AudioComponent))

(event OnAudioPlaybackPercent(MM_ThemeTrack)
  (params (PlayingSoundWave :type Sound%20Wave%20Object%20Reference) (PlaybackPercent :type Float%20%28single-precision%29))
  (if (>= PlaybackPercent 0.94)
    (Audio|Components|Audio|FadeOut (Variables|Default|GetMM_ThemeTrack) 4.25 0.0 "Linear" :!class /Script/Engine.AudioComponent)))

(event EventBeginPlay
  (bind _mm_themetrack (Variables|Default|GetMM_ThemeTrack))
  (Audio|Components|Audio|Play _mm_themetrack 0.0)
  (Audio|Components|Audio|FadeIn _mm_themetrack 4.0 1.0 0.0 "Linear" :!class /Script/Engine.AudioComponent))

(event Collision|EventActorBeginOverlap
  (params (OtherActor :type Actor%20Object%20Reference)))

(event EventTick
  (params (DeltaSeconds :type Float%20%28single-precision%29)))

(fn ConstructionScript)