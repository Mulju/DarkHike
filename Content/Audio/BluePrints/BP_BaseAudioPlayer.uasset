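; BP_BaseAudioPlayer is a base sound actor that plays looped or player-triggered audio.
; Tick restarts looping sounds, optionally after fixed or randomized delays, waiting for a first overlap when triggered.
; Player overlaps with an assigned or auto-spawned TriggerBox start looping or play one-shots, limited by trigger count or random chance.
; BeginPlay reconciles option flags, seeds the random stream from the clock and can override the sound's submix.
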(event OnActorBeginOverlap(Trigger)
  (params (OverlappedActor :type Actor%20Object%20Reference) (OtherActor :type Actor%20Object%20Reference))
  (bind _baseaudiocomponent (Variables|Components|Audio|GetBaseAudioComponent))
  (bind _returnvalue (Audio|Components|Audio|GetPlayState _baseaudiocomponent))
  (bind _returnvalue_2 (!= 0 _returnvalue))
  (bind _output_get (Variables|State|SetIs%20Overlapper%20Player (== OtherActor (Game|GetPlayerCharacter 0))))
  (if _output_get
    (if (Variables|Definition|Behaviour|Looping|GetLoop)
      (Variables|State|SetFirst%20Trigger false)
      (elif (Variables|Definition|Behaviour|Triggering|GetTrigger%20Random)
        (if (Variables|Definition|Behaviour|Triggering|GetTrigger%20Times%20Random)
          (if (> (Variables|Definition|Behaviour|Triggering|GetNumber%20Triggers) 0) :!label _label
            (if _returnvalue_2
              (Audio|Components|Audio|Play (Variables|Components|Audio|GetBaseAudioComponent) 0.0)
              (if (Variables|State|GetFirst%20Trigger)
                (Variables|State|SetFirst%20Trigger false))
              (Variables|Definition|Behaviour|Triggering|SetNumber%20Triggers (- (Variables|Definition|Behaviour|Triggering|GetNumber%20Triggers) 1)))
            (else
              (if (Math|Random|RandomBoolfromStream (Variables|Default|GetRandomStream)) :!label _label_2
                (if (<= (Variables|Definition|Behaviour|Triggering|GetNumber%20Triggers) 0)
                  (if _returnvalue_2
                    (Audio|Components|Audio|Play (Variables|Components|Audio|GetBaseAudioComponent) 0.0))))))
          (else
            (goto _label_2)))
        (elif (Variables|Definition|Behaviour|Triggering|GetTrigger%20Times%20Random)
          (goto _label)
          (elif (< (Variables|Definition|Behaviour|Triggering|GetNumber%20Triggers) 0)
            (if _returnvalue_2 :!label _label_3
              (Audio|Components|Audio|Play (Variables|Components|Audio|GetBaseAudioComponent) 0.0)
              (Variables|Definition|Behaviour|Triggering|SetNumber%20Triggers (- (Variables|Definition|Behaviour|Triggering|GetNumber%20Triggers) 1))
              (Variables|State|SetFirst%20Trigger false))
            (elif (Variables|State|GetIs%20Overlapper%20Player)
              (if (> (Variables|Definition|Behaviour|Triggering|GetNumber%20Triggers) 0)
                (goto _label_3)
                (else
                  (Development|PrintString "Trigger Count has reached zero" false))))))))))

(event OnAudioFinished(BaseAudioComponent))

(event OnAudioPlaybackPercent(BaseAudioComponent)
  (params (PlayingSoundWave :type Sound%20Wave%20Object%20Reference) (PlaybackPercent :type Float%20%28single-precision%29))
  (bind _baseaudiocomponent (Variables|Components|Audio|GetBaseAudioComponent))
  (if (>= PlaybackPercent 1.0)
    (if (!= (Variables|Definition|Behaviour|Looping|GetLoop) true)
      (if (== (Audio|Components|Audio|GetPlayState _baseaudiocomponent) 0) :!label _label
        (Audio|Components|Audio|Stop _baseaudiocomponent))
      (elif (Variables|Definition|Behaviour|Looping|GetLoop%20Delayed)
        (goto _label)))))

(event EventBeginPlay
  (bind _self self)
  (bind _trigger_random (Variables|Definition|Behaviour|Triggering|GetTrigger%20Random))
  (bind _returnvalue (Transformation|GetActorLocation _self))
  (Utilities|FlowControl|Sequence
    (:then_0
      (Audio|Components|Audio|Stop (Variables|Components|Audio|GetBaseAudioComponent)))
    (:then_1
      (Variables|State|SetFirstPlay true))
    (:then_2
      (CallFunction|TimeBasedSeed) ; Generate Random Seed From Current Time
    )
    (:then_3
      ;[1 1 1] Loop Delayed=Loop
      (if (not (Variables|Definition|Behaviour|Looping|GetLoop))
        (if (Variables|Definition|Behaviour|Looping|GetLoop%20Delayed)
          (Variables|Definition|Behaviour|Looping|SetLoop true))))
    (:then_4
      ;[1 1 1] TriggerBox=IsTrigger
      (if (!= (Variables|Components|Default|GetTrigger) 0)
        (Variables|Definition|Behaviour|Triggering|SetIsTriggered true)))
    (:then_5
      ;[1 1 1] IsTrigger=TriggerBox
      (if (Variables|Definition|Behaviour|Triggering|GetIsTriggered)
        (if (== (Variables|Components|Default|GetTrigger) 0)
          (bind _returnvalue_2 (Game|SpawnActorfromClass "/Script/Engine.TriggerBox" (Math|Transform|MakeTransform (Math|Vector|MakeVector (+ (.x _returnvalue) 6e+01) (.y _returnvalue) (.z _returnvalue)) "0, 0, 0" "3.000000,3.000000,3.000000") "Undefined" "MultiplyWithRoot" 0 0))
          (bind _output_get (Variables|Components|Default|SetTrigger _returnvalue_2))
          (Rendering|SetActorHiddenInGame _output_get false))))
    (:then_6
      (if (== _trigger_random (Variables|Definition|Behaviour|Triggering|GetTrigger%20Times%20Random))
        (if _trigger_random
          (Variables|Definition|Behaviour|Triggering|SetNumber%20Triggers 0 :!label _label)
          (Variables|Definition|Behaviour|Triggering|SetTrigger%20Times%20Random false))
        (elif _trigger_random
          (goto _label))))
    (:then_7
      ;[1 1 1] Override Sound Submix
      (if (Variables|Definition|Override|GetOR%20Submix)
        (Variables|/Script/Engine.SoundBase|SetSoundSubmixObject (Variables|/Script/Engine.AudioComponent|GetSound (Variables|Components|Audio|GetBaseAudioComponent)) (Variables|Components|Audio|GetOverride%20Submix))))))

(event Collision|EventActorBeginOverlap
  (params (OtherActor :type Actor%20Object%20Reference)))

(event EventTick
  (params (DeltaSeconds :type Float%20%28single-precision%29))
  (bind _baseaudiocomponent (Variables|Components|Audio|GetBaseAudioComponent))
  (bind _returnvalue (Audio|Components|Audio|GetPlayState _baseaudiocomponent))
  (bind _returnvalue_2 (!= 0 _returnvalue))
  (Utilities|FlowControl|Sequence
    (:then_0
      (if (Variables|Definition|Behaviour|Looping|GetLoop)
        (if (Variables|Definition|Behaviour|Triggering|GetIsTriggered)
          (if (Variables|State|GetFirst%20Trigger)
            (Development|PrintString "Looping not triggered yet" false)
            (else
              ;[1 1 1] Loop, Delay, Random Delay
              (if (Variables|Definition|Behaviour|Looping|GetLoop) :!label _label
                (if (Variables|Definition|Behaviour|Looping|GetLoop%20Delayed)
                  (if (Variables|Definition|Behaviour|Looping|GetRandomize%20Loop%20Delay%20Interval)
                    (if _returnvalue_2
                      (bind _randominterval (CallFunction|VariedDelayTime))
                      (Utilities|FlowControl|Delay _randominterval)
                      (Audio|Components|Audio|Play (Variables|Components|Audio|GetBaseAudioComponent) 0.0))
                    (elif (Variables|State|GetFirstPlay)
                      (if _returnvalue_2 :!label _label_2
                        (Audio|Components|Audio|Play (Variables|Components|Audio|GetBaseAudioComponent) 0.0)
                        (Variables|State|SetFirstPlay false))
                      (elif _returnvalue_2
                        (Utilities|FlowControl|Delay (Variables|Definition|Behaviour|Values|GetDelay%20Seconds))
                        (Audio|Components|Audio|Play (Variables|Components|Audio|GetBaseAudioComponent) 0.0))))
                  (else
                    (goto _label_2))))))
          (else
            (goto _label)))))))

(fn ConstructionScript)

(fn TimeBasedSeed
  (bind _returnvalue (Math|DateTime|Now))
  (Variables|Default|SetRandomStream (Math|Random|MakeRandomStream (+ (+ (.year _returnvalue) (.month _returnvalue) (.day _returnvalue)) (/ (+ (.hour _returnvalue) (.minute _returnvalue) (.second _returnvalue) (.millisecond _returnvalue)) 60))))
  (return))

(fn VariedDelayTime
  (return (Math|Random|RandomFloatinRangefromStream (Variables|Default|GetRandomStream) (- (Variables|Definition|Behaviour|Values|GetDelay%20Seconds) (Variables|Definition|Behaviour|Values|GetDelay%20Variation)) (+ (Variables|Definition|Behaviour|Values|GetDelay%20Seconds) (Variables|Definition|Behaviour|Values|GetDelay%20Variation)))))