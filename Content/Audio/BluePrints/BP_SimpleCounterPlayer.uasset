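; BP_SimpleCounterPlayer is an actor that plays its audio once after repeated Interact presses near a trigger box.
; It enables its own input and counts presses made within a fixed distance of TriggerBox, playing Audio when the count reaches ActivationNum.
; Any actor leaving the trigger resets the count.
; An overlap flag tracks BP_Player entry, but the press check uses distance instead.
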(event OnActorBeginOverlap(TriggerBox)
  (params (OverlappedActor :type Actor%20Object%20Reference) (OtherActor :type Actor%20Object%20Reference))
  (Utilities|Casting|CastToBP_Player OtherActor)
  (Variables|Default|SetIsOverlappingTrigger true))

(event OnActorEndOverlap(TriggerBox)
  (params (OverlappedActor :type Actor%20Object%20Reference) (OtherActor :type Actor%20Object%20Reference))
  (Variables|Default|SetIsOverlappingTrigger false)
  (Variables|Default|SetCounter 0))

(event EventBeginPlay
  (Audio|Components|Audio|Stop (Variables|Default|GetAudio))
  (Input|EnableInput (Game|GetPlayerController 0)))

(event Collision|EventActorBeginOverlap
  (params (OtherActor :type Actor%20Object%20Reference)))

(event EventTick
  (params (DeltaSeconds :type Float%20%28single-precision%29)))

(event Input|ActionEvents|InputActionInteract
  (params (Key :type Key%20Structure :default "None"))
  (:Pressed
    (if (<= (Transformation|GetDistanceTo (Variables|Default|GetTriggerBox) (Game|GetPlayerCharacter 0)) 3e+02)
      (Variables|Default|SetCounter (+ (Variables|Default|GetCounter) 1))
      (if (== (Variables|Default|GetCounter) (Variables|Default|GetActivationNum))
        (if (not (Variables|Default|GetHasActivated))
          (Audio|Components|Audio|Play (Variables|Default|GetAudio) 0.0)
          (Variables|Default|SetHasActivated true))))))

(fn ConstructionScript)