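; BP_AmbieFinalPlayer is an actor that plays the ending music, picking a good or evil track based on the player's score.
; On BeginPlay it casts the game instance to GameInstanceDarkHike and reads GoodBadScore.
; A score at or above the threshold sets the Audio component to Loppumusa_Good, otherwise Loppumusa_EVIL, then starts playback from the beginning.
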(event EventBeginPlay
  (bind _audio (Variables|Default|GetAudio))
  (bind _asgame_instance_dark_hike (Utilities|Casting|CastToGameInstanceDarkHike (Game|GetGameInstance)))
  (if (>= (Variables|/Script/DarkHike.GameInstanceDarkHike|GetgoodBadScore _asgame_instance_dark_hike) 2)
    (Audio|Components|Audio|SetSound _audio "/Game/Audio/Map3/Loppumusa_Good.Loppumusa_Good")
    (else
      (Audio|Components|Audio|SetSound _audio "/Game/Audio/Map3/Loppumusa_EVIL.Loppumusa_EVIL")))
  (Audio|Components|Audio|Play (Variables|Default|GetAudio) 0.0))

(event Collision|EventActorBeginOverlap
  (params (OtherActor :type Actor%20Object%20Reference))
  (|CallParentFunction OtherActor) ; This node is disabled and will not be called.\nDrag off pins to build functionality.
)

(event EventTick
  (params (DeltaSeconds :type Float%20%28single-precision%29))
  (|CallParentFunction DeltaSeconds) ; This node is disabled and will not be called.\nDrag off pins to build functionality.
)

(fn ConstructionScript
  (|CallParentFunction))