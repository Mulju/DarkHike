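; BP_GraveGate is an interactable graveyard gate that opens only for a player carrying the graveyard key.
; A box overlap tracks the player, and pressing Interact queries their key inventory.
; With the key, it plays the open sequence and hides the prompt widget; otherwise it rattles and steps through dialogue lines, ignoring movement input until they end.
; A GateClose event reverses the open sequence.
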(event OnComponentBeginOverlap(Box)
  (params (OverlappedComponent :type Primitive%20Component%20Object%20Reference) (OtherActor :type Actor%20Object%20Reference) (OtherComp :type Primitive%20Component%20Object%20Reference) (OtherBodyIndex :type Integer) (bFromSweep :type Boolean) (SweepResult :type Hit%20Result%20Structure%20%28by%20ref%29))
  (bind _asbp_player (Utilities|Casting|CastToBP_Player OtherActor))
  (Utilities|IsValid _asbp_player
    (:Is%20Valid
      (Variables|Default|SetOverlappingPlayer _asbp_player)
      (Development|PrintString "Begun graveyard gate overlap")
      (Variables|Default|SetIsOverlapping true))))

(event OnComponentEndOverlap(Box)
  (params (OverlappedComponent :type Primitive%20Component%20Object%20Reference) (OtherActor :type Actor%20Object%20Reference) (OtherComp :type Primitive%20Component%20Object%20Reference) (OtherBodyIndex :type Integer))
  (bind _asbp_player (Utilities|Casting|CastToBP_Player OtherActor))
  (Utilities|IsValid _asbp_player
    (:Is%20Valid
      (Development|PrintString "Ended graveyard gate overlap")
      (Variables|Default|SetIsOverlapping false))))

(event Custom|Event%20GateOpen
  (Development|PrintString "mee")
  (if (Variables|Default|GetbOpen)
    (Development|PrintString "Gate Already Open")
    (else
      (Class|ActorSequenceComponent|PlaySequence (Variables|Default|GetGateOpen))
      (Variables|Default|SetbOpen true))))

(event Custom|Event%20GateClose
  (if (Variables|Default|GetbOpen)
    (Class|MovieSceneSequencePlayer|PlayReverse (Variables|/Script/ActorSequence.ActorSequenceComponent|GetSequencePlayer (Variables|Default|GetGateOpen)))
    (Variables|Default|SetbOpen false)
    (else
      (Development|PrintString "Gate Already Open"))))

(event Collision|EventActorBeginOverlap
  (params (OtherActor :type Actor%20Object%20Reference)))

(event EventTick
  (params (DeltaSeconds :type Float%20%28single-precision%29)))

(event EventBeginPlay
  (Input|EnableInput (Game|GetPlayerController 0))
  (Variables|Default|SetIsInteractable true))

(event Input|ActionEvents|InputActionInteract
  (params (Key :type Key%20Structure :default "None"))
  (:Pressed
    (if (Variables|Default|GetIsOverlapping)
      (if (.bSuccess (Default|QueryInventory (Variables|/Game/Code/Character/BP_Player.BP_Player_C|GetKeyItemInventory (Variables|Default|GetOverlappingPlayer)) "graveyardkey" 1))
        (CallFunction|EventGateOpen)
        (Variables|Default|SetIsInteractable false)
        (Rendering|SetVisibility (Variables|Default|GetModularWidget) false false)
        (else
          (CallFunction|ShowDialogue)
          (Class|ActorSequenceComponent|PlaySequence (Variables|Default|GetGateRattle)))))))

(fn ConstructionScript)

(fn ShowDialogue
  (bind _result (Math|Integer|IncrementInt (Variables|Default|GetTalkIndex))
    (:%20%20
      (Development|PrintString (Utilities|String|ToString(Integer) _result))
      (if (< (Variables|Default|GetTalkIndex) (Utilities|Array|Length (Variables|Default|GetDialogue)))
        (Development|PrintString "Went true")
        (Input|SetIgnoreMoveInput (Game|GetPlayerController 0) true)
        (Variables|Default|GetUI
          (:then
            _)
          (:else
            (bind _returnvalue (UserInterface|CreateWidget "/Game/Blueprints/UI-Widgets/W_DialogueBase.W_DialogueBase_C" (Game|GetPlayerController 0)))
            (bind _output_get (Variables|Default|SetUI _returnvalue))
            (UserInterface|Viewport|AddtoViewport _output_get 0)))
        (Class|DialogueWidget|SetDialogueText (Variables|Default|GetUI) (Utilities|Array|Get(acopy) (Variables|Default|GetDialogue) (Variables|Default|GetTalkIndex)))
        (else
          (Development|PrintString "Went false")
          (Widget|RemovefromParent (Variables|Default|GetUI))
          (Variables|Default|SetTalkIndex -1)
          (Variables|Default|SetUI 0)
          (Input|SetIgnoreMoveInput (Game|GetPlayerController 0) false))))))