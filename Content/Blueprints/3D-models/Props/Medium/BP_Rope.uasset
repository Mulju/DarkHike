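; BP_Rope is an interactable rope prop with a key item mesh and chandelier audio.
; BeginPlay stops the audio, stores the mesh's starting height and binds the rope interaction event, which plays the audio.
; While IsActivated is set, Tick integrates FallingAcceleration into velocity and moves the mesh vertically, but only while its world Z is at or below a hardcoded threshold.
; The stored height is unused here, and IsActivated is not set in this graph.
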(event Custom|On%20Rope%20Interact
  (Audio|Components|Audio|Play (Variables|Default|GetChandelierAudio) 0.0))

(event EventBeginPlay
  (EventDispatchers|BindEventtoOnRopeInteractionEvent (delegate Custom|On%20Rope%20Interact))
  (Audio|Components|Audio|Stop (Variables|Default|GetChandelierAudio))
  (Variables|Default|SetOriginalLocationZ (.Z (Math|Vector|BreakVector (Transformation|GetWorldLocation (Variables|Default|GetKeyItemMesh))))))

(event Collision|EventActorBeginOverlap
  (params (OtherActor :type Actor%20Object%20Reference)))

(event EventTick
  (params (DeltaSeconds :type Float%20%28single-precision%29))
  (bind _keyitemmesh (Variables|Default|GetKeyItemMesh))
  (bind _returnvalue (Transformation|GetWorldLocation _keyitemmesh))
  (bind (_x _y _z) (Math|Vector|BreakVector _returnvalue))
  (if (Variables|Default|GetbIsActivated)
    (if (<= _z -1.2e+04)
      (bind _output_get (Variables|Default|SetCurrentVelocity (+ (Variables|Default|GetCurrentVelocity) (* DeltaSeconds (Variables|Default|GetFallingAcceleration)))))
      (Transformation|SetWorldLocation (Variables|Default|GetKeyItemMesh) (Math|Vector|MakeVector _x _y (+ _z (* _output_get DeltaSeconds))) false false))))

(fn ConstructionScript)