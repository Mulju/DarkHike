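; Altar prop that, while IsStairs is set, moves a referenced Stairs actor to its raised location and then clears a blocker.
; Tick adds a fixed step to the lerp alpha and interpolates from the stairs' current location, so motion accelerates then settles and depends on frame rate.
; Within tolerance of the target, DisableBlocker destroys the single Altar-tagged BP_BoxBlocker.
; Tick keeps calling it afterwards, printing a warning once none remains.
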(event EventBeginPlay)

(event Collision|EventActorBeginOverlap
  (params (OtherActor :type Actor%20Object%20Reference)))

(event EventTick
  (params (DeltaSeconds :type Float%20%28single-precision%29))
  (bind _stairs (Variables|Default|GetStairs))
  (bind _stairlocationup (Variables|Default|GetStairLocationUp))
  (if (Variables|Default|GetIsStairs)
    (Utilities|IsValid _stairs
      (:Is%20Valid
        (Variables|Default|SetLerpVariable (Math|Float|Clamp(Float) (+ (Variables|Default|GetLerpVariable) 0.001)))
        (Transformation|SetActorLocation _stairs (Math|Vector|Lerp(Vector) (Transformation|GetActorLocation (Variables|Default|GetStairs)) _stairlocationup (Variables|Default|GetLerpVariable)) false false)
        (if (Utilities|Operators|EqualEqual (Transformation|GetActorLocation (Variables|Default|GetStairs)) _stairlocationup 0.1)
          (CallFunction|DisableBlocker)))
      (:Is%20Not%20Valid
        (Development|PrintString "Stairs reference is not valid")))))

(fn ConstructionScript)

(fn DisableBlocker
  (bind _outactors (Actor|GetAllActorsOfClasswithTag "/Game/Code/Mechanics/BP_BoxBlocker.BP_BoxBlocker_C" "Altar"))
  (if (== (Utilities|Array|Length _outactors) 1)
    (Actor|DestroyActor (Utilities|Array|Get(acopy) _outactors))
    (else
      (Development|PrintString "The altar didn't find 1 blocker"))))