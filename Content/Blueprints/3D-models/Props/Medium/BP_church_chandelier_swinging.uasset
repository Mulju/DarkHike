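; Church chandelier prop Blueprint meant to swing gently by rotating itself on Tick.
; It lerps the actor from PivotPoint's world rotation toward WantedRotation, using an alpha that climbs to one and never resets.
; On arrival it picks a ±2 degree target, but the forward-vector X test cannot equal 2, so only the positive target is chosen.
; The alpha is printed every frame for debugging.
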(event EventTick
  (params (DeltaSeconds :type Float%20%28single-precision%29))
  (if (Utilities|Operators|EqualEqual (Transformation|GetWorldRotation (Variables|Default|GetPivotPoint self)) (Variables|Default|GetWantedRotation) 0.0)
    (if (== (.X (Math|Vector|BreakVector (Math|Rotator|GetRotationXVector (Variables|Default|GetWantedRotation)))) 2.0)
      (Variables|Default|SetWantedRotation "0.000000,0.000000,-2.000000")
      (else
        (Variables|Default|SetWantedRotation "0.000000,0.000000,2.000000")))
    (else
      (Variables|Default|SetLerpRotation (Math|Float|Clamp(Float) (+ (Variables|Default|GetLerpRotation) 0.001)))
      (Transformation|SetActorRotation (Math|Rotator|Lerp(Rotator) (Transformation|GetWorldRotation (Variables|Default|GetPivotPoint self)) (Variables|Default|GetWantedRotation) (Variables|Default|GetLerpRotation)))))
  (Development|PrintString (Utilities|String|ToString(Float) (Variables|Default|GetLerpRotation))))

(fn ConstructionScript)