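; Collision volume for the maze prop that enables wall walking for the player while they are inside it.
; Entering WallWalkBox sets CanWallWalk on BP_Player, allows walking off ledges and lowers the movement component's max step height.
; Leaving the box disables wall walking and ledge walk-off and raises the step height again, using hard-coded values rather than saved ones.
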(event OnComponentBeginOverlap(WallWalkBox)
  (params (OverlappedComponent :type Primitive%20Component%20Object%20Reference) (OtherActor :type Actor%20Object%20Reference) (OtherComp :type Primitive%20Component%20Object%20Reference) (OtherBodyIndex :type Integer) (bFromSweep :type Boolean) (SweepResult :type Hit%20Result%20Structure%20%28by%20ref%29))
  (bind _asbp_player (Utilities|Casting|CastToBP_Player OtherActor)
    (:then
      (Utilities|IsValid _asbp_player
        (:Is%20Valid
          (Variables|/Game/Code/Character/BP_Player.BP_Player_C|SetbCanWallWalk _asbp_player true)
          (Variables|/Script/Engine.CharacterMovementComponent|SetbCanWalkOffLedges (Variables|/Script/Engine.Character|GetCharacterMovement _asbp_player) true)
          (Variables|/Script/Engine.CharacterMovementComponent|SetMaxStepHeight (Variables|/Script/Engine.Character|GetCharacterMovement _asbp_player) 1e+01))))
    (:CastFailed
      (Development|PrintString "Player Cast Failed"))))

(event OnComponentEndOverlap(WallWalkBox)
  (params (OverlappedComponent :type Primitive%20Component%20Object%20Reference) (OtherActor :type Actor%20Object%20Reference) (OtherComp :type Primitive%20Component%20Object%20Reference) (OtherBodyIndex :type Integer))
  (bind _asbp_player (Utilities|Casting|CastToBP_Player OtherActor)
    (:then
      (Utilities|IsValid _asbp_player
        (:Is%20Valid
          (Variables|/Game/Code/Character/BP_Player.BP_Player_C|SetbCanWallWalk _asbp_player false)
          (Variables|/Script/Engine.CharacterMovementComponent|SetbCanWalkOffLedges (Variables|/Script/Engine.Character|GetCharacterMovement _asbp_player) false)
          (Variables|/Script/Engine.CharacterMovementComponent|SetMaxStepHeight (Variables|/Script/Engine.Character|GetCharacterMovement _asbp_player) 45.0))))
    (:CastFailed
      (Development|PrintString "Player Cast Failed"))))

(fn ConstructionScript)