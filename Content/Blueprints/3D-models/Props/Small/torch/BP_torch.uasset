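; Torch prop that lights and goes out in response to a linked pressure plate trigger.
; On BeginPlay it binds to the OnPlatePressed dispatcher of its Trigger reference, if one is valid.
; The event's IsActive flag activates or deactivates the Flames effect and switches the point light intensity between lit and zero.
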(event Custom|OnPlatePressed
  (params (IsActive :type Boolean))
  (bind _flames (Variables|Default|GetFlames))
  (bind _pointlight (Variables|Default|GetPointLight))
  (if IsActive
    (Components|Activation|Activate _flames false)
    (Rendering|Components|Light|SetIntensity _pointlight 1e+03)
    (else
      (Components|Activation|Deactivate _flames)
      (Rendering|Components|Light|SetIntensity _pointlight 0.0))))

(event EventBeginPlay
  (bind _trigger (Variables|Default|GetTrigger))
  (Utilities|IsValid _trigger
    (:Is%20Valid
      (EventDispatchers|BindEventtoOnPlatePressed _trigger (EventDispatchers|CreateEvent :!event Custom|OnPlatePressed)))))

(fn ConstructionScript)