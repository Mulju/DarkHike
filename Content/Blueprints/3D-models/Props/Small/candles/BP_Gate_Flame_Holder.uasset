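; Gate flame holder prop whose blue flame, point light and audio switch on or off together with player proximity.
; It binds to the player-enter event of a referenced Trigger in both the construction script and BeginPlay, when that Trigger is valid.
; OnPlayerProximity's boolean drives all three effects.
; At BeginPlay the flame effect is activated for one tick, then deactivated.
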(event Custom|OnPlayerProximity
  (params (IsActive :type Boolean))
  (bind _audio (Variables|Default|GetAudio))
  (bind _pointlight (Variables|Default|GetPointLight))
  (bind _flamesblue (Variables|Default|GetFlamesBlue))
  (if IsActive
    (Components|Activation|Activate _flamesblue false)
    (Rendering|Components|Light|SetIntensity _pointlight 5e+03)
    (Audio|Components|Audio|Play _audio 0.0)
    (else
      (Components|Activation|Deactivate _flamesblue)
      (Rendering|Components|Light|SetIntensity _pointlight 0.0)
      (Audio|Components|Audio|Stop _audio))))

(event EventBeginPlay
  (bind _flamesblue (Variables|Default|GetFlamesBlue))
  (bind _trigger (Variables|Default|GetTrigger))
  (Components|Activation|Activate _flamesblue false)
  (Utilities|FlowControl|DelayUntilNextTick)
  (Components|Activation|Deactivate _flamesblue)
  (Utilities|IsValid _trigger
    (:Is%20Valid
      (EventDispatchers|BindEventtoOnPlayerEnter _trigger (EventDispatchers|CreateEvent :!event Custom|OnPlayerProximity)))))

(event Collision|EventActorBeginOverlap
  (params (OtherActor :type Actor%20Object%20Reference)))

(event EventTick
  (params (DeltaSeconds :type Float%20%28single-precision%29)))

(fn ConstructionScript
  (bind _trigger (Variables|Default|GetTrigger))
  (Utilities|IsValid _trigger
    (:Is%20Valid
      (EventDispatchers|BindEventtoOnPlayerEnter _trigger (EventDispatchers|CreateEvent :!event Custom|OnPlayerProximity)))))