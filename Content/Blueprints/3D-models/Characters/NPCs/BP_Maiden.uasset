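; BP_Maiden is an NPC Blueprint that handles player interaction dialogue for the Maiden character.
; On BeginPlay it binds its handler to the character interaction event.
; The first interaction plays the Maiden's 2D sound, enables the talk flag and advances the dialogue counter.
; Later interactions advance the counter until it equals the dialogue length, then the next one resets the conversation state.
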(event Custom|OnMaidenInteraction
  (if (Variables|Default|GetFirstInteract)
    (Audio|PlaySound2D "/Game/Audio/Character/Maiden/Maiden.Maiden" 1.0 1.0 0.0 0 0)
    (Variables|Default|SetDialogueCounter (+ (Variables|Default|GetDialogueCounter) 1))
    (Variables|Default|SetFirstInteract false)
    (Variables|Default|SetACanTalk true)
    (elif (== (Variables|Default|GetDialogueCounter) (Variables|Default|GetDialogueLength))
      (Variables|Default|SetFirstInteract true)
      (Variables|Default|SetDialogueCounter 0)
      (Variables|Default|SetACanTalk false)
      (else
        (Variables|Default|SetDialogueCounter (+ (Variables|Default|GetDialogueCounter) 1))))))

(event EventBeginPlay
  (EventDispatchers|BindEventtoOnCharacterInteractionEvent (delegate Custom|OnMaidenInteraction)))

(event Collision|EventActorBeginOverlap
  (params (OtherActor :type Actor%20Object%20Reference)))

(event EventTick
  (params (DeltaSeconds :type Float%20%28single-precision%29)))

(fn ConstructionScript)