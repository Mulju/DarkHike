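; Generic soul NPC that turns to face the player during interaction.
; Each tick it calls RotateWidgetToCamera and, if interacted with and rotation is enabled, blends its yaw toward the player character.
; Otherwise it blends yaw back toward its original rotation.
; Both blends share a clamped alpha that rises by a fixed, frame-rate-dependent step and is not reset in this graph.
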(event EventBeginPlay)

(event EventTick
  (params (DeltaSeconds :type Float%20%28single-precision%29))
  (bind _self self)
  (Class|InteractableCharacter|RotateWidgettoCamera)
  (if (and (Variables|Default|GetbIsInteractedWith) (Variables|Default|GetbIsRotatingCharacter))
    (Variables|Default|SetLerpVariable (Math|Float|Clamp(Float) (+ (Variables|Default|GetLerpVariable) 0.01)))
    (Transformation|SetActorRotation (Math|Rotator|MakeRotator 0.0 0.0 (.Yaw (Math|Rotator|BreakRotator (Math|Rotator|Lerp(Rotator) (Transformation|GetActorRotation _self) (Math|Rotator|FindLookatRotation (Transformation|GetActorLocation _self) (Transformation|GetActorLocation (Game|GetPlayerCharacter 0))) (Variables|Default|GetLerpVariable))))))
    (else
      (Variables|Default|SetLerpVariable (Math|Float|Clamp(Float) (+ (Variables|Default|GetLerpVariable) 0.01)))
      (Transformation|SetActorRotation (Math|Rotator|MakeRotator 0.0 0.0 (.Yaw (Math|Rotator|BreakRotator (Math|Rotator|Lerp(Rotator) (Transformation|GetActorRotation self) (Variables|Default|GetOriginalRotation) (Variables|Default|GetLerpVariable)))))))))

(fn ConstructionScript)