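; Priest NPC that plays dialogue when the player interacts with it and reacts to a heard sound.
; Interaction starts the dialogue player, with a timer re-enabling speech after a short cooldown.
; Tick polls IsHearingSound, which nothing here sets, then shakes the camera and clears the flag.
; The same reaction switches the Box collision of a lone BP_ViewChange tagged "Key" to overlap-all.
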(event Custom|On%20Interaction%20Event
  (if (Variables|Default|GetCanSpeak)
    (Audio|Components|Audio|Play (Variables|Default|GetPriestDialoguePlayer) 0.0)
    (Variables|Default|SetCanSpeak false)
    (Utilities|Time|SetTimerbyFunctionName 0 "TimerSetCanSpeak" 4.09)))

(event EventBeginPlay
  (Audio|Components|Audio|Stop (Variables|Default|GetPriestDialoguePlayer))
  (EventDispatchers|BindEventtoOnCharacterInteractionEvent (delegate Custom|On%20Interaction%20Event)))

(event Collision|EventActorBeginOverlap
  (params (OtherActor :type Actor%20Object%20Reference)))

(event EventTick
  (params (DeltaSeconds :type Float%20%28single-precision%29))
  (if (Variables|Default|GetbIsHearingSound)
    (Camera|PlayWorldCameraShake "/Game/Code/Mechanics/BP_CameraShake.BP_CameraShake_C" (Camera|GetCameraLocation (Game|GetPlayerCameraManager 0)) 0.0 3e+03)
    (bind _outactors (Actor|GetAllActorsOfClasswithTag "/Game/Code/Mechanics/BP_ViewChange.BP_ViewChange_C" "Key"))
    (if (== (Utilities|Array|Length _outactors) 1)
      (Collision|SetCollisionProfileName (Variables|/Game/Code/Mechanics/BP_ViewChange.BP_ViewChange_C|GetBox (Utilities|Array|Get(acopy) _outactors)) "OverlapAllDynamic" true :!class /Script/Engine.PrimitiveComponent))
    (Variables|Default|SetbIsHearingSound false)))

(fn ConstructionScript)

(fn TimerSetCanSpeak
  (Variables|Default|SetCanSpeak true))