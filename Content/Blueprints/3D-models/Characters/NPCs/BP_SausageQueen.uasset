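; BP_SausageQueen is a dialogue NPC that rises from a dive when the player first approaches and dives again after talking.
; BeginPlay picks one of two dialogues from the GameInstance karma score.
; Trigger overlap plays audio and enables interaction; the interaction event counts lines, drives talk and dive flags, and destroys PlayerBLocker on first talk.
; BoxComp overlaps blend the camera to the queen before the first talk and back to the pawn on exit.
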(event OnComponentBeginOverlap(BoxComp)
  (params (OverlappedComponent :type Primitive%20Component%20Object%20Reference) (OtherActor :type Actor%20Object%20Reference) (OtherComp :type Primitive%20Component%20Object%20Reference) (OtherBodyIndex :type Integer) (bFromSweep :type Boolean) (SweepResult :type Hit%20Result%20Structure%20%28by%20ref%29))
  (if (Variables|Default|GetFirstTalk)
    (if (== OtherActor (Game|GetPlayerCharacter 0))
      (Game|Player|SetViewTargetwithBlend (Game|GetPlayerController 0) self (Variables|Default|GetBlendTimeFromPlayer) "VTBlend_EaseInOut" (Variables|Default|GetBlendVariable) false)
      (Development|PrintString "Entered box"))))

(event OnComponentEndOverlap(BoxComp)
  (params (OverlappedComponent :type Primitive%20Component%20Object%20Reference) (OtherActor :type Actor%20Object%20Reference) (OtherComp :type Primitive%20Component%20Object%20Reference) (OtherBodyIndex :type Integer))
  (if (Variables|Default|GetFirstTalk)
    _
    (else
      (Utilities|FlowControl|DoOnce false
        (:Completed
          _))))
  (if (== OtherActor (Game|GetPlayerCharacter 0))
    (Game|Player|SetViewTargetwithBlend (Game|GetPlayerController 0) (Pawn|GetControlledPawn (Game|GetPlayerController 0)) (Variables|Default|GetBlendTimeFromPlayer) "VTBlend_EaseInOut" (Variables|Default|GetBlendVariable) false)
    (Development|PrintString "Exited box")))

(event OnComponentBeginOverlap(Trigger)
  (params (OverlappedComponent :type Primitive%20Component%20Object%20Reference) (OtherActor :type Actor%20Object%20Reference) (OtherComp :type Primitive%20Component%20Object%20Reference) (OtherBodyIndex :type Integer) (bFromSweep :type Boolean) (SweepResult :type Hit%20Result%20Structure%20%28by%20ref%29))
  (if (Variables|Default|GetFirstTalk)
    (if (== OtherActor (Game|GetPlayerCharacter 0))
      (Audio|Components|Audio|SetSound (Variables|Default|GetSausageAudio) "/Game/Audio/Character/Sausage/Merimakkara.Merimakkara")
      (if (Variables|Default|GetCanPlayBublu)
        (Audio|Components|Audio|Play (Variables|Default|GetSausageAudio) 0.0))
      (Utilities|FlowControl|Delay 2.2)
      (Variables|Sausage|ABP|SetACanDiveUp true)
      (Variables|Sausage|ABP|SetACanDiveDown false)
      (Variables|Default|SetCanPlayBublu false)
      (Utilities|FlowControl|Delay 0.2)
      (Variables|Default|SetbInteractionEnabled true))))

(event OnComponentEndOverlap(Trigger)
  (params (OverlappedComponent :type Primitive%20Component%20Object%20Reference) (OtherActor :type Actor%20Object%20Reference) (OtherComp :type Primitive%20Component%20Object%20Reference) (OtherBodyIndex :type Integer)))

(event Custom|Sausage%20Interaction%20Event
  (Utilities|FlowControl|Sequence
    (:then_0
      (if (Variables|Default|GetFirstTalk)
        (Variables|Default|SetInteractionCounter 0)
        (Variables|Default|SetFirstTalk false)
        (Variables|Sausage|ABP|SetACanTalk true)
        (Audio|Components|Audio|SetSound (Variables|Default|GetSausageAudio) "/Game/Audio/Character/Sausage/BLoodqueen.BLoodqueen")
        (Audio|Components|Audio|Play (Variables|Default|GetSausageAudio) 0.0)
        (bind _playerblocker (Variables|Default|GetPlayerBLocker)
          (:then
            (Actor|DestroyActor _playerblocker))
          (:else))))
    (:then_1
      (bind _returnvalue (Class|InteractableCharacter|GetDialogueArrayLength (Variables|Default|GetDialoguesIndex)))
      (if (== _returnvalue (Variables|Default|GetInteractionCounter))
        (Variables|Default|SetFirstTalk false)
        (Variables|Sausage|ABP|SetACanTalk false)
        (Variables|Sausage|ABP|SetACanDiveUp false)
        (Variables|Sausage|ABP|SetACanDiveDown true)
        (Variables|Default|SetbInteractionEnabled false)
        (Audio|Components|Audio|SetSound (Variables|Default|GetSausageAudio) "/Game/Audio/Character/Sausage/Merimakkara.Merimakkara")
        (Audio|Components|Audio|Play (Variables|Default|GetSausageAudio) 0.0)
        (Variables|Default|SetCanPlayBublu false)))
    (:then_2
      (Variables|Default|SetInteractionCounter (+ (Variables|Default|GetInteractionCounter) 1)))))

(event EventBeginPlay
  (Utilities|FlowControl|Sequence
    (:then_0
      (EventDispatchers|BindEventtoOnCharacterInteractionEvent (delegate Custom|Sausage%20Interaction%20Event)))
    (:then_1
      (Components|Activation|Activate (Variables|Default|GetSausageAudio) true)
      (Audio|Components|Audio|Stop (Variables|Default|GetSausageAudio)))
    (:then_2
      ;[1 1 1] Set Dialogue Based On Karma
      (bind _asgi_dark_hike (Utilities|Casting|CastToGI_DarkHike (Game|GetGameInstance)))
      (if (>= (Variables|/Script/DarkHike.GameInstanceDarkHike|GetgoodBadScore _asgi_dark_hike) 2)
        (Variables|Default|SetDialoguesIndex 0)
        (else
          (Variables|Default|SetDialoguesIndex 1))))
    (:then_3
      (Variables|Default|SetbInteractionEnabled false))))

(event Collision|EventActorBeginOverlap
  (params (OtherActor :type Actor%20Object%20Reference)))

(event EventTick
  (params (DeltaSeconds :type Float%20%28single-precision%29)))

(fn ConstructionScript)