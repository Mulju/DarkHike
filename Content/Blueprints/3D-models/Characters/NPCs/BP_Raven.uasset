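; BP_Raven is the raven NPC, which plays alert and dialogue audio for the player.
; Front and back trigger actors play the alert when the player overlaps, then disable their own collision.
; An interaction event sets ACanTalk and, within range with CanPlay true, plays dialogue, disables the back trigger and starts a timer to clear ACanTalk.
; The logic that sets CanPlay is disconnected, and the playback-percent event is empty.
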(event OnActorBeginOverlap(Trigger_AlertFront)
  (params (OverlappedActor :type Actor%20Object%20Reference) (OtherActor :type Actor%20Object%20Reference))
  (if (== OtherActor (Game|GetPlayerCharacter 0))
    (Audio|Components|Audio|Play (Variables|Default|GetRavenAlertPlayer) 0.0)
    (Collision|SetActorEnableCollision (Variables|Default|GetTrigger_AlertFront) false)))

(event OnActorBeginOverlap(Trigger_AlertBack)
  (params (OverlappedActor :type Actor%20Object%20Reference) (OtherActor :type Actor%20Object%20Reference))
  (if (== OtherActor (Game|GetPlayerCharacter 0))
    (Audio|Components|Audio|Play (Variables|Default|GetRavenAlertPlayer) 0.0)
    (Collision|SetActorEnableCollision (Variables|Default|GetTrigger_AlertBack) false)))

(event OnAudioPlaybackPercent(RavenDialoguePlayer)
  (params (PlayingSoundWave :type Sound%20Wave%20Object%20Reference) (PlaybackPercent :type Float%20%28single-precision%29)))

(event Custom|Raven%20On%20Interact
  (Utilities|FlowControl|Sequence
    (:then_0
      (Variables|Default|SetACanTalk true))
    (:then_1
      (if (<= (Transformation|GetDistanceTo (Game|GetPlayerCharacter 0) self) 4e+02)
        (if (Variables|Default|GetCanPlay)
          (Audio|Components|Audio|Play (Variables|Default|GetRavenDialoguePlayer) 0.0)
          (Collision|SetActorEnableCollision (Variables|Default|GetTrigger_AlertBack) false)
          (Utilities|Time|SetTimerbyFunctionName 0 "DelayedACanTalk" 2.0))))))

(event EventBeginPlay
  (Audio|Components|Audio|Stop (Variables|Default|GetRavenAlertPlayer))
  (Audio|Components|Audio|Stop (Variables|Default|GetRavenDialoguePlayer))
  (EventDispatchers|BindEventtoOnCharacterInteractionEvent (delegate Custom|Raven%20On%20Interact)))

(event EventTick
  (params (DeltaSeconds :type Float%20%28single-precision%29)))

(fn ConstructionScript)

(fn DelayedACanTalk
  (Variables|Default|SetACanTalk false))