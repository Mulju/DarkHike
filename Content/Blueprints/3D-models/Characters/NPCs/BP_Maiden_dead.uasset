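; Dead Maiden NPC that the player can interact with to step through a dialogue.
; On BeginPlay it sets ACanDead and binds its handler to the character interaction event.
; The first interaction plays the Maiden 2D sound and enables talking, and later ones advance a dialogue counter.
; An interaction at the dialogue's length resets the state, so the conversation can replay.
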(event Custom|OnMaidenInteraction
  (if (Variables|Default|GetFirstInteract_0)
    (Audio|PlaySound2D "/Game/Audio/Character/Maiden/Maiden.Maiden" 1.0 1.0 0.0 0 0)
    (Variables|Default|SetDialogueCounter_0 (+ (Variables|Default|GetDialogueCounter_0) 1))
    (Variables|Default|SetFirstInteract_0 false)
    (Variables|Default|SetACanTalk_0 true)
    (elif (== (Variables|Default|GetDialogueCounter_0) (Variables|Default|GetDialogueLength_0))
      (Variables|Default|SetFirstInteract_0 true)
      (Variables|Default|SetDialogueCounter_0 0)
      (Variables|Default|SetACanTalk_0 false)
      (else
        (Variables|Default|SetDialogueCounter_0 (+ (Variables|Default|GetDialogueCounter_0) 1))))))

(event EventBeginPlay
  (Variables|Default|SetACanDead true)
  (EventDispatchers|BindEventtoOnCharacterInteractionEvent (delegate Custom|OnMaidenInteraction)))

(event Collision|EventActorBeginOverlap
  (params (OtherActor :type Actor%20Object%20Reference)))

(event EventTick
  (params (DeltaSeconds :type Float%20%28single-precision%29)))

(fn ConstructionScript)